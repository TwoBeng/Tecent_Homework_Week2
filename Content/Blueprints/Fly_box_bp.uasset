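; Flying box target that shuttles back and forth along local X and scores for the player who damages it.
; Each Tick calls a server move event that offsets the Cube, flipping direction after a fixed step count.
; For network sync, it stores the world location and calls a client event that applies it.
; Damage increments the instigator's MyPlayerState score, destroying the box only if that cast fails.
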(event `self.ReceiveTick`
  (params (DeltaSeconds :type "Float (single-precision)"))
  ;[1 1 1] 网络同步移动
  (`self.sever_move`))

(event `sever_move`
  ;[1 1 1] 网络同步移动
  (if (`self.isTurn`)
    (`SceneComponent.K2_AddLocalOffset` (`self.Cube`) (10.0 0.0 0.0) false false)
    (else
      (`SceneComponent.K2_AddLocalOffset` (`self.Cube`) (-10.0 0.0 0.0) false false)))
  (`/Engine/EditorBlueprintResources/StandardMacros.IncrementInt` (`self.count`)
    (:`  `
      (set `self.location` (`SceneComponent.K2_GetComponentLocation` (`self.Cube`)))
      (`self.client_move`)
      (if (>= (`self.count`) 80)
        (set `self.count` 0)
        (set `self.isTurn` (not (`self.isTurn`)))))))

(event `client_move`
  ;[1 1 1] 网络同步移动
  (`SceneComponent.K2_SetWorldLocation` (`self.Cube`) (`self.location`) false false))

(event `self.ReceiveAnyDamage`
  (params (Damage :type "Float (single-precision)") (DamageType :type "DamageType Object Reference") (InstigatedBy :type "Controller Object Reference") (DamageCauser :type "Actor Object Reference"))
  (bind _asmy_player_state (cast `/Game/Blueprints/MyPlayerState` (`Controller.PlayerState` InstigatedBy))
    (:`then`
      (`/Game/Blueprints/MyPlayerState.IncrementScore` _asmy_player_state))
    (:`CastFailed`
      (`self.K2_DestroyActor`))))

(fn `UserConstructionScript`)